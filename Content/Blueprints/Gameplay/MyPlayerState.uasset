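; Player state holding a character's loadout and stats: two weapon slots, held gun, 5.56 and 7.62 ammo, health, energy, equipment, fashion items and backpack contents.
; Getters expose each value, while setters and add/remove functions update it and fire a matching change event for listeners.
; AddItem merges health and boost items into an existing stack of the same type and ID, adding a new entry otherwise.
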(fn `AddEquipment`
  (params (Equipment :type "/Game/Blueprints/GeneralItems/ItemBase Object Reference"))
  (`KismetArrayLibrary.Array_Add` (`self.Equipments`) Equipment)
  (`self.Event_EquipmentsChanged` Equipment true))

(fn `AddFashion`
  (params (Fashion :type "/Game/Blueprints/GeneralItems/ItemBase Object Reference"))
  (`KismetArrayLibrary.Array_Add` (`self.Fashions`) Fashion)
  (`self.Event_FashionsChanged` Fashion true))

(fn `AddItem`
  (params (Item :type "/Game/Blueprints/GeneralItems/ItemBase Object Reference"))
  (locals (IsFound :type Boolean))
  (bind _itemtype (`/Game/Blueprints/GeneralItems/ItemBase.ItemType` Item))
  (bind _item (`local.Item`))
  (bind _item_2 (`local.Item`))
  ;[1 1 1] If the item is health or boost then possibly stack items
  (if (or (`|EnumEquality` _itemtype "NewEnumerator3") (`|EnumEquality` _itemtype "NewEnumerator4"))
    (for _array_element (`self.ItemsInBackpack`)
      (if (and (`|EnumEquality` (`/Game/Blueprints/GeneralItems/ItemBase.ItemType` _array_element) (`/Game/Blueprints/GeneralItems/ItemBase.ItemType` _item_2)) (== (`/Game/Blueprints/GeneralItems/ItemBase.ID` _array_element) (`/Game/Blueprints/GeneralItems/ItemBase.ID` _item_2)))
        (set `/Game/Blueprints/GeneralItems/ItemBase.Amount` (+ (`/Game/Blueprints/GeneralItems/ItemBase.Amount` _array_element) (`/Game/Blueprints/GeneralItems/ItemBase.Amount` (`local.Item`))) _array_element)
        (set `local.IsFound` true)
        (`self.Event_ItemsChanged` _array_element true)
        (break))))
  ;[1 1 1] If no previous boost or health, or if not boost or health
  (if (not (`local.IsFound`))
    (`KismetArrayLibrary.Array_Add` (`self.ItemsInBackpack`) _item)
    (`self.Event_ItemsChanged` _item true)))

(fn `GetAmmo556`
  (returns (Amount :type Integer))
  (return (`self.Ammo556`)))

(fn `GetAmmo762`
  (returns (Amount :type Integer))
  (return (`self.Ammo762`)))

(fn `GetEnergyPoint`
  (returns (Value :type "Float (double-precision)"))
  (return (`self.EnergyPoint`)))

(fn `GetEquipments`
  (returns (Equipments :type "Array of /Game/Blueprints/GeneralItems/ItemBase Object Reference"))
  (return (`self.Equipments`)))

(fn `GetFashions`
  (returns (Fashions :type "Array of /Game/Blueprints/GeneralItems/ItemBase Object Reference"))
  (return (`self.Fashions`)))

(fn `GetHealthPoint`
  (returns (Value :type "Float (double-precision)"))
  (return (`self.HealthPoint`)))

(fn `GetHoldGun`
  (returns (Weapon :type "/Game/Blueprints/GeneralItems/Equipments/ItemWeapon Object Reference"))
  (return (`self.HoldGun`)))

(fn `GetItemsInBackpack`
  (returns (Items :type "Array of /Game/Blueprints/GeneralItems/ItemBase Object Reference"))
  (return (`self.ItemsInBackpack`)))

(fn `GetWeapon1`
  (returns (Weapon :type "/Game/Blueprints/GeneralItems/Equipments/ItemWeapon Object Reference"))
  (return (`self.Weapon1`)))

(fn `GetWeapon2`
  (returns (Weapon :type "/Game/Blueprints/GeneralItems/Equipments/ItemWeapon Object Reference"))
  (return (`self.Weapon2`)))

(fn `RemoveEquipment`
  (params (Equipment :type "/Game/Blueprints/GeneralItems/ItemBase Object Reference"))
  (returns (Removed :type Boolean))
  (bind _returnvalue (`KismetArrayLibrary.Array_RemoveItem` (`self.Equipments`) Equipment))
  (`self.Event_EquipmentsChanged` Equipment)
  (return _returnvalue))

(fn `RemoveFashion`
  (params (Fashion :type "/Game/Blueprints/GeneralItems/ItemBase Object Reference"))
  (returns (Removed :type Boolean))
  (bind _returnvalue (`KismetArrayLibrary.Array_RemoveItem` (`self.Fashions`) Fashion))
  (`self.Event_FashionsChanged` Fashion)
  (return _returnvalue))

(fn `RemoveItem`
  (params (Item :type "/Game/Blueprints/GeneralItems/ItemBase Object Reference"))
  (returns (Removed :type Boolean))
  (bind _returnvalue (`KismetArrayLibrary.Array_RemoveItem` (`self.ItemsInBackpack`) Item))
  (`self.Event_ItemsChanged` Item)
  (return _returnvalue))

(fn `SetAmmo556`
  (params (Value :type Integer))
  (set `self.Ammo556` Value)
  (`self.Event_AmmoChanged`))

(fn `SetAmmo762`
  (params (Value :type Integer))
  (set `self.Ammo762` Value)
  (`self.Event_AmmoChanged`))

(fn `SetEnergyPoint`
  (params (Value :type "Float (double-precision)"))
  (set `self.EnergyPoint` Value)
  (`self.Event_EnergyPointChanged` Value))

(fn `SetHealthPoint`
  (params (Value :type "Float (double-precision)"))
  (set `self.HealthPoint` Value)
  (`self.Event_HealthPointChanged` Value))

(fn `SetHoldGun`
  (params (Weapon :type "/Game/Blueprints/GeneralItems/Equipments/ItemWeapon Object Reference"))
  (bind _output_get (set `self.HoldGun` Weapon))
  (`/Engine/EditorBlueprintResources/StandardMacros.IsValid` _output_get
    (:`Is Valid`
      (`self.Event_WeaponChanged` _output_get (`/Game/Blueprints/GeneralItems/Equipments/ItemWeapon.Position` _output_get) true))
    (:`Is Not Valid`
      (`self.Event_WeaponChanged` _output_get "NewEnumerator0" true) ; if invalid, don't set position
    )))

(fn `SetWeapon1`
  (params (Weapon :type "/Game/Blueprints/GeneralItems/Equipments/ItemWeapon Object Reference"))
  (bind _output_get (set `self.Weapon1` Weapon))
  (`self.Event_WeaponChanged` _output_get "NewEnumerator0"))

(fn `SetWeapon2`
  (params (Weapon :type "/Game/Blueprints/GeneralItems/Equipments/ItemWeapon Object Reference"))
  (bind _output_get (set `self.Weapon2` Weapon))
  (`self.Event_WeaponChanged` _output_get "NewEnumerator1"))

(fn `UserConstructionScript`)