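; Game mode that procedurally spawns loot pickups across the map on BeginPlay.
; Each DT_ItemGroup_Location row spawns an ItemGroup, filled with a random count of distinct item types and IDs, mostly weighted by data-table percentages expanded into shuffled arrays.
; A generated weapon adds its matching ammo, displacing a non-weapon item.
; Items spawn as type-specific pickup actors at unused group transforms, with serial numbers from MyGameInstance.
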(event `self.ReceiveBeginPlay`
  (bind _asmy_game_instance (cast `/Game/Blueprints/Gameplay/MyGameInstance` (`GameplayStatics.GetGameInstance`)))
  (set `self.MyGameInstanceRef` _asmy_game_instance)
  (`self.GenerateItems`))

(fn `GenerateItems`
  (locals (ItemGroupRef :type "/Game/Blueprints/GeneralItems/ItemGroup Object Reference") (ItemTypesGenerated :type "Array of /Game/Blueprints/Data/Enum/E_ItemType Enum") (ItemTypeandIDArr :type "Array of /Game/Blueprints/Data/TableStructures/ItemGenerations/ST_ItemType_and_ID Structure") (SpawnType :type "/Game/Blueprints/Data/Enum/E_ItemType Enum") (SpawnID :type Name) (UsedLocations :type "Array of Transform Structure") (SpawnLocation :type "Transform Structure") (ItemsObject :type "Array of /Game/Blueprints/GeneralItems/Pickups/PickupBase Object Reference"))
  ;[1 1 1] Get all items in group locations
  (bind _outrownames (`DataTableFunctionLibrary.GetDataTableRowNames` "/Game/Blueprints/Data/DataTables/Items/DT_ItemGroup_Location.DT_ItemGroup_Location"))
  (for _array_element _outrownames
    (`KismetSystemLibrary.PrintString` "process a group")
    (bind _returnvalue (`|GetDataTableRow` "/Game/Blueprints/Data/DataTables/Items/DT_ItemGroup_Location.DT_ItemGroup_Location" _array_element)
      (:`then`
        ;[1 1 1] Spawn a group
        (bind _returnvalue_2 (`|SpawnActorFromClass` "/Game/Blueprints/GeneralItems/ItemGroup.ItemGroup_C" (`KismetMathLibrary.MakeTransform` (`.Location_3_67C81EDA47C56A3E8F1D738E73E9CD32` (break `/Game/Blueprints/Data/TableStructures/Items/ST_ItemGroup_Location` _returnvalue))) "Undefined" "OverrideRootScale" null null))
        (set `local.ItemGroupRef` _returnvalue_2)
        ;[1 1 1] For each item group, add quanity number of random types (no same type in one group)
        (bind _quantity (`self.RandomItemNumber`))
        (for _ (range 1 (+ _quantity 1))
          (bind _itemtype (`self.RandomItemType` :!label _label))
          (if (== (`KismetArrayLibrary.Array_Find` (`local.ItemTypesGenerated`) _itemtype) -1)
            (`KismetArrayLibrary.Array_Add` (`local.ItemTypesGenerated`) _itemtype)
            (else
              (goto _label))))
        ;[1 1 1] Generate a item based on type
        (for _array_element_2 (`local.ItemTypesGenerated`)
          (bind _item (`self.RandomItemID` _array_element_2))
          (`KismetArrayLibrary.Array_Add` (`local.ItemTypeandIDArr`) _item))
        (`KismetArrayLibrary.Array_Clear` (`local.ItemTypesGenerated`))
        ;[1 1 1] Create Ammo item in the group for weapon if a weapon is generated
        (for _array_element_3 (`local.ItemTypeandIDArr`)
          (bind (_type _id) (break `/Game/Blueprints/Data/TableStructures/ItemGenerations/ST_ItemType_and_ID` _array_element_3))
          (if (`|EnumEquality` _type "NewEnumerator0")
            (bind _returnvalue_3 (`|GetDataTableRow` "/Game/Blueprints/Data/DataTables/Items/DT_Item_Weapon.DT_Item_Weapon" _id)
              (:`then`
                (`KismetArrayLibrary.Array_Add` (`local.ItemTypeandIDArr`) (make `/Game/Blueprints/Data/TableStructures/ItemGenerations/ST_ItemType_and_ID` "NewEnumerator2" (`.UseAmmoID_12_59009020437530EB32597AADEC4B422D` (break `/Game/Blueprints/Data/TableStructures/Items/ST_Item_Weapon` _returnvalue_3))))
                ;[1 1 1] This ammo item replaces an item that is not the weapon in the group
                (for (_array_element_4 _array_index) (`local.ItemTypeandIDArr`)
                  (if (`|EnumInequality` (`.Type_3_73F501DC49A5907C9186FDA4E4432FFB` (break `/Game/Blueprints/Data/TableStructures/ItemGenerations/ST_ItemType_and_ID` _array_element_4)) "NewEnumerator0")
                    (`KismetArrayLibrary.Array_Remove` (`local.ItemTypeandIDArr`) _array_index)
                    (break)))))))
        ;[1 1 1] At this point, a group of items has been created as types and ids
        (for _array_element_5 (`local.ItemTypeandIDArr`)
          (bind (_type_2 _id_2) (break `/Game/Blueprints/Data/TableStructures/ItemGenerations/ST_ItemType_and_ID` _array_element_5))
          (set `local.SpawnType` _type_2)
          (set `local.SpawnID` _id_2)
          (`|ExecutionSequence`
            (:`then_0`
              ;[1 1 1] Random location
              (bind _location (`self.RandomLocation` (`/Game/Blueprints/GeneralItems/ItemGroup.GetAllTransform` (`local.ItemGroupRef`)) :!label _label_2))
              (if (== (`KismetArrayLibrary.Array_Find` (`local.UsedLocations`) _location) -1)
                (bind _output_get (set `local.SpawnLocation` _location))
                (`KismetArrayLibrary.Array_Add` (`local.UsedLocations`) _output_get)
                (else
                  (goto _label_2))))
            (:`then_1`
              (switch `/Game/Blueprints/Data/Enum/E_ItemType` (`local.SpawnType`)
                (:`NewEnumerator0`
                  (bind _returnvalue_4 (`|SpawnActorFromClass` "/Game/Blueprints/GeneralItems/Pickups/PickupWeapon.PickupWeapon_C" (`local.SpawnLocation`) "Undefined" "OverrideRootScale" null 0 (`local.SpawnID`) (`/Game/Blueprints/Gameplay/MyGameInstance.GenerateSN` (`self.MyGameInstanceRef`)) 1 null))
                  (`KismetArrayLibrary.Array_Add` (`local.ItemsObject`) _returnvalue_4))
                (:`NewEnumerator1`
                  (bind _returnvalue_5 (`|SpawnActorFromClass` "/Game/Blueprints/GeneralItems/Pickups/PickupWeaponAcc.PickupWeaponAcc_C" (`local.SpawnLocation`) "Undefined" "OverrideRootScale" null (`local.SpawnID`) (`/Game/Blueprints/Gameplay/MyGameInstance.GenerateSN` (`self.MyGameInstanceRef`)) 1 null))
                  (`KismetArrayLibrary.Array_Add` (`local.ItemsObject`) _returnvalue_5))
                (:`NewEnumerator2`
                  (bind _returnvalue_6 (`|SpawnActorFromClass` "/Game/Blueprints/GeneralItems/Pickups/PickupAmmo.PickupAmmo_C" (`local.SpawnLocation`) "Undefined" "OverrideRootScale" null (`local.SpawnID`) (`/Game/Blueprints/Gameplay/MyGameInstance.GenerateSN` (`self.MyGameInstanceRef`)) 0 null)) ; ammo has amount = 0
                  (`KismetArrayLibrary.Array_Add` (`local.ItemsObject`) _returnvalue_6))
                (:`NewEnumerator3`
                  (bind _returnvalue_7 (`|SpawnActorFromClass` "/Game/Blueprints/GeneralItems/Pickups/PickupHealth.PickupHealth_C" (`local.SpawnLocation`) "Undefined" "OverrideRootScale" null (`local.SpawnID`) (`/Game/Blueprints/Gameplay/MyGameInstance.GenerateSN` (`self.MyGameInstanceRef`)) 1 null))
                  (`KismetArrayLibrary.Array_Add` (`local.ItemsObject`) _returnvalue_7))
                (:`NewEnumerator4`
                  (bind _returnvalue_8 (`|SpawnActorFromClass` "/Game/Blueprints/GeneralItems/Pickups/PickupBoost.PickupBoost_C" (`local.SpawnLocation`) "Undefined" "OverrideRootScale" null (`local.SpawnID`) (`/Game/Blueprints/Gameplay/MyGameInstance.GenerateSN` (`self.MyGameInstanceRef`)) 1 null))
                  (`KismetArrayLibrary.Array_Add` (`local.ItemsObject`) _returnvalue_8))
                (:`NewEnumerator5`
                  (bind _returnvalue_9 (`|SpawnActorFromClass` "/Game/Blueprints/GeneralItems/Pickups/PickupEquipment.PickupEquipment_C" (`local.SpawnLocation`) "Undefined" "OverrideRootScale" null (`local.SpawnID`) (`/Game/Blueprints/Gameplay/MyGameInstance.GenerateSN` (`self.MyGameInstanceRef`)) 1 null :!label _label_3))
                  (`KismetArrayLibrary.Array_Add` (`local.ItemsObject`) _returnvalue_9))
                (:`NewEnumerator6`
                  (goto _label_3))
                (:`NewEnumerator7`
                  (goto _label_3))
                (:`NewEnumerator8`
                  (bind _returnvalue_10 (`|SpawnActorFromClass` "/Game/Blueprints/GeneralItems/Pickups/PickupFashion.PickupFashion_C" (`local.SpawnLocation`) "Undefined" "OverrideRootScale" null (`local.SpawnID`) (`/Game/Blueprints/Gameplay/MyGameInstance.GenerateSN` (`self.MyGameInstanceRef`)) 1 null))
                  (`KismetArrayLibrary.Array_Add` (`local.ItemsObject`) _returnvalue_10))))))
        ;;[1 1 1 1 14] Need this at the end of each group process
        (`KismetArrayLibrary.Array_Clear` (`local.ItemTypeandIDArr`))))))

(fn `RandomItemID`
  (params (ItemType :type "/Game/Blueprints/Data/Enum/E_ItemType Enum" :default "NewEnumerator0"))
  (returns (Item :type "/Game/Blueprints/Data/TableStructures/ItemGenerations/ST_ItemType_and_ID Structure"))
  (locals (Arr :type "Array of /Game/Blueprints/Data/TableStructures/ItemGenerations/ST_ItemType_and_ID Structure"))
  (bind _arr (`local.Arr`))
  (`|ExecutionSequence`
    (:`then_0`
      (switch `/Game/Blueprints/Data/Enum/E_ItemType` ItemType
        (:`NewEnumerator0`
          (bind _outrownames (`DataTableFunctionLibrary.GetDataTableRowNames` "/Game/Blueprints/Data/DataTables/Items/DT_Item_Weapon.DT_Item_Weapon"))
          (for _array_element _outrownames
            (bind _returnvalue (`|GetDataTableRow` "/Game/Blueprints/Data/DataTables/Items/DT_Item_Weapon.DT_Item_Weapon" _array_element)
              (:`then`
                (for _ (range 1 (+ (`.ProbPercent_96_F3CF757D46C07E12A480219FC67AE1A6` (break `/Game/Blueprints/Data/TableStructures/Items/ST_Item_Weapon` _returnvalue)) 1))
                  (`KismetArrayLibrary.Array_Add` (`local.Arr`) (make `/Game/Blueprints/Data/TableStructures/ItemGenerations/ST_ItemType_and_ID` "NewEnumerator0" _array_element)))))))
        (:`NewEnumerator1`
          (bind _outrownames_2 (`DataTableFunctionLibrary.GetDataTableRowNames` "/Game/Blueprints/Data/DataTables/Items/DT_Item_WeaponAcc.DT_Item_WeaponAcc"))
          (for _array_element_2 _outrownames_2
            ;[1 1 1] Not 100?
            (`KismetArrayLibrary.Array_Add` (`local.Arr`) (make `/Game/Blueprints/Data/TableStructures/ItemGenerations/ST_ItemType_and_ID` "NewEnumerator1" _array_element_2))))
        (:`NewEnumerator2`
          (bind _outrownames_3 (`DataTableFunctionLibrary.GetDataTableRowNames` "/Game/Blueprints/Data/DataTables/Items/DT_Item_Ammo.DT_Item_Ammo"))
          (for _array_element_3 _outrownames_3
            (bind _returnvalue_2 (`|GetDataTableRow` "/Game/Blueprints/Data/DataTables/Items/DT_Item_Ammo.DT_Item_Ammo" _array_element_3)
              (:`then`
                (for _ (range 1 (+ (`.ProbPercent_18_C2E6A6D2470701BC2E9773879E30C009` (break `/Game/Blueprints/Data/TableStructures/Items/ST_Item_Ammo` _returnvalue_2)) 1))
                  (`KismetArrayLibrary.Array_Add` (`local.Arr`) (make `/Game/Blueprints/Data/TableStructures/ItemGenerations/ST_ItemType_and_ID` "NewEnumerator2" _array_element_3)))))))
        (:`NewEnumerator3`
          (bind _outrownames_4 (`DataTableFunctionLibrary.GetDataTableRowNames` "/Game/Blueprints/Data/DataTables/Items/DT_Item_Health.DT_Item_Health"))
          (for _array_element_4 _outrownames_4
            (bind _returnvalue_3 (`|GetDataTableRow` "/Game/Blueprints/Data/DataTables/Items/DT_Item_Health.DT_Item_Health" _array_element_4)
              (:`then`
                (for _ (range 1 (+ (`.ProbPercent_21_A5ACBC654F2B733E20EAC88E3950833C` (break `/Game/Blueprints/Data/TableStructures/Items/ST_Item_Health` _returnvalue_3)) 1))
                  (`KismetArrayLibrary.Array_Add` (`local.Arr`) (make `/Game/Blueprints/Data/TableStructures/ItemGenerations/ST_ItemType_and_ID` "NewEnumerator3" _array_element_4)))))))
        (:`NewEnumerator4`
          (bind _outrownames_5 (`DataTableFunctionLibrary.GetDataTableRowNames` "/Game/Blueprints/Data/DataTables/Items/DT_Item_Boost.DT_Item_Boost"))
          (for _array_element_5 _outrownames_5
            (bind _returnvalue_4 (`|GetDataTableRow` "/Game/Blueprints/Data/DataTables/Items/DT_Item_Boost.DT_Item_Boost" _array_element_5)
              (:`then`
                (for _ (range 1 (+ (`.ProbPercent_21_4EA6CEDB41F9595EC43B71B270CF624F` (break `/Game/Blueprints/Data/TableStructures/Items/ST_Item_Boost` _returnvalue_4)) 1))
                  (`KismetArrayLibrary.Array_Add` (`local.Arr`) (make `/Game/Blueprints/Data/TableStructures/ItemGenerations/ST_ItemType_and_ID` "NewEnumerator4" _array_element_5)))))))
        (:`NewEnumerator5`
          (bind _outrownames_6 (`DataTableFunctionLibrary.GetDataTableRowNames` "/Game/Blueprints/Data/DataTables/Items/DT_Item_Equipment.DT_Item_Equipment"))
          (for _array_element_6 _outrownames_6
            (bind _returnvalue_5 (`|GetDataTableRow` "/Game/Blueprints/Data/DataTables/Items/DT_Item_Equipment.DT_Item_Equipment" _array_element_6)
              (:`then`
                (bind (_name _type _staticmesh _icon _thumbnails _capacity _probpercent) (break `/Game/Blueprints/Data/TableStructures/Items/ST_Item_Equipment` _returnvalue_5))
                (if (`|EnumEquality` _type "NewEnumerator5")
                  (for _ (range 1 (+ _probpercent 1))
                    (`KismetArrayLibrary.Array_Add` (`local.Arr`) (make `/Game/Blueprints/Data/TableStructures/ItemGenerations/ST_ItemType_and_ID` "NewEnumerator5" _array_element_6))))))))
        (:`NewEnumerator6`
          (bind _outrownames_7 (`DataTableFunctionLibrary.GetDataTableRowNames` "/Game/Blueprints/Data/DataTables/Items/DT_Item_Equipment.DT_Item_Equipment"))
          (for _array_element_7 _outrownames_7
            (bind _returnvalue_6 (`|GetDataTableRow` "/Game/Blueprints/Data/DataTables/Items/DT_Item_Equipment.DT_Item_Equipment" _array_element_7)
              (:`then`
                (bind (_name_2 _type_2 _staticmesh_2 _icon_2 _thumbnails_2 _capacity_2 _probpercent_2) (break `/Game/Blueprints/Data/TableStructures/Items/ST_Item_Equipment` _returnvalue_6))
                (if (`|EnumEquality` _type_2 "NewEnumerator6")
                  (for _ (range 1 (+ _probpercent_2 1))
                    (`KismetArrayLibrary.Array_Add` (`local.Arr`) (make `/Game/Blueprints/Data/TableStructures/ItemGenerations/ST_ItemType_and_ID` "NewEnumerator6" _array_element_7))))))))
        (:`NewEnumerator7`
          (bind _outrownames_8 (`DataTableFunctionLibrary.GetDataTableRowNames` "/Game/Blueprints/Data/DataTables/Items/DT_Item_Equipment.DT_Item_Equipment"))
          (for _array_element_8 _outrownames_8
            (bind _returnvalue_7 (`|GetDataTableRow` "/Game/Blueprints/Data/DataTables/Items/DT_Item_Equipment.DT_Item_Equipment" _array_element_8)
              (:`then`
                (bind (_name_3 _type_3 _staticmesh_3 _icon_3 _thumbnails_3 _capacity_3 _probpercent_3) (break `/Game/Blueprints/Data/TableStructures/Items/ST_Item_Equipment` _returnvalue_7))
                (if (`|EnumEquality` _type_3 "NewEnumerator7")
                  (for _ (range 1 (+ _probpercent_3 1))
                    (`KismetArrayLibrary.Array_Add` (`local.Arr`) (make `/Game/Blueprints/Data/TableStructures/ItemGenerations/ST_ItemType_and_ID` "NewEnumerator7" _array_element_8))))))))
        (:`NewEnumerator8`
          (bind _outrownames_9 (`DataTableFunctionLibrary.GetDataTableRowNames` "/Game/Blueprints/Data/DataTables/Items/DT_Item_Fashion.DT_Item_Fashion"))
          (for _array_element_9 _outrownames_9
            (if (and (!= _array_element_9 "1") (!= _array_element_9 "4"))
              (`KismetArrayLibrary.Array_Add` (`local.Arr`) (make `/Game/Blueprints/Data/TableStructures/ItemGenerations/ST_ItemType_and_ID` "NewEnumerator8" _array_element_9)))))))
    (:`then_1`
      (`KismetArrayLibrary.Array_Shuffle` _arr)
      (return (`|GetArrayItem` _arr (`KismetMathLibrary.RandomIntegerInRange` 0 (- (`KismetArrayLibrary.Array_Length` (`local.Arr`)) 1)))))))

(fn `RandomItemNumber`
  (returns (Quantity :type Integer))
  (locals (Arr :type "Array of Integer") (`3` :type Integer) (`4` :type Integer) (`5` :type Integer))
  ;[1 1 1] For each row name, index into to row name
  (bind _outrownames (`DataTableFunctionLibrary.GetDataTableRowNames` "/Game/Blueprints/Data/DataTables/ItemGeneration/DT_QuantityProbability.DT_QuantityProbability"))
  (for _array_element _outrownames
    (bind _returnvalue (`|GetDataTableRow` "/Game/Blueprints/Data/DataTables/ItemGeneration/DT_QuantityProbability.DT_QuantityProbability" _array_element)
      (:`then`
        (bind (_percent _quantity) (break `/Game/Blueprints/Data/TableStructures/ItemGenerations/ST_QuantityProbability` _returnvalue))
        (for _ (range 1 (+ _percent 1))
          (`KismetArrayLibrary.Array_Add` (`local.Arr`) _quantity)))))
  (for _array_element_2 (`local.Arr`)
    (switch `int` _array_element_2
      (:`3`
        (`/Engine/EditorBlueprintResources/StandardMacros.IncrementInt` (`local.3`)))
      (:`4`
        (`/Engine/EditorBlueprintResources/StandardMacros.IncrementInt` (`local.4`)))
      (:`5`
        (`/Engine/EditorBlueprintResources/StandardMacros.IncrementInt` (`local.5`)))))
  (`KismetArrayLibrary.Array_Shuffle` (`local.Arr`))
  (return (`|GetArrayItem` (`local.Arr`) (`KismetMathLibrary.RandomIntegerInRange` 0 99))))

(fn `RandomItemType`
  (returns (ItemType :type "/Game/Blueprints/Data/Enum/E_ItemType Enum"))
  (locals (Arr :type "Array of /Game/Blueprints/Data/Enum/E_ItemType Enum"))
  (bind _outrownames (`DataTableFunctionLibrary.GetDataTableRowNames` "/Game/Blueprints/Data/DataTables/ItemGeneration/DT_ItemTypeProb.DT_ItemTypeProb"))
  (for _array_element _outrownames
    (bind _returnvalue (`|GetDataTableRow` "/Game/Blueprints/Data/DataTables/ItemGeneration/DT_ItemTypeProb.DT_ItemTypeProb" _array_element)
      (:`then`
        (bind (_percent _type) (break `/Game/Blueprints/Data/TableStructures/ItemGenerations/ST_ItemTypeProb` _returnvalue))
        (for _ (range 1 (+ _percent 1))
          (`KismetArrayLibrary.Array_Add` (`local.Arr`) _type)))))
  (`KismetArrayLibrary.Array_Shuffle` (`local.Arr`))
  (return (`|GetArrayItem` (`local.Arr`) (`KismetMathLibrary.RandomIntegerInRange` 0 99))))

(fn `RandomLocation`
  (params (Available :type "Array of Transform Structure"))
  (returns (Location :type "Transform Structure"))
  (return (`|GetArrayItem` Available (`KismetMathLibrary.RandomIntegerInRange` 0 (- (`KismetArrayLibrary.Array_Length` Available) 1)))))

(fn `UserConstructionScript`)